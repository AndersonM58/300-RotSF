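; Hinged door actor that swings open and closed in response to Trigger and Toggle events.
; Construction script sizes the door mesh from width, height and thickness, adding instanced hinges at even spacing and an optional three-piece frame.
; AllowTriggersToToggleToo makes both events flip the state; otherwise Trigger is ignored and Toggle follows its boolean.
; A timeline, rate-scaled to the set opening time, plays or reverses to drive the hinge's yaw.
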(event `/Game/Blueprints/Interface/ITriggerOrToggle.Trigger`
  (if (`self.Allow triggers to toggle too`)
    ;[1 1 1] FLIP FLOP
    (set `self.IsOpen` (not (`self.IsOpen`)) :!label _label)
    (`TimelineComponent.SetPlayRate` (`self.Open The Door`) (/ (`TimelineComponent.GetTimelineLength` (`self.Open The Door`)) (`self.How long does it take to open?`)) :!label _label_2)
    (if (`self.IsOpen`)
      (bind (_direction _percent) (`Timeline|Open The Door` :!label _label_3)
        (:`Update`
          (`SceneComponent.K2_SetRelativeRotation` (`self.Hinge`) (`KismetMathLibrary.MakeRotator` 0.0 0.0 (* _percent (`self.How many degees to open`) -1.0)) false false)))
      (else
        (goto _label_3 :!via `Reverse`)))))

(event `/Game/Blueprints/Interface/ITriggerOrToggle.Toggle`
  (params (IsNowOn :type Boolean))
  (if (`self.Allow triggers to toggle too`)
    (goto _label)
    (else
      ;[1 1 1] Slave to Boolean
      (set `self.IsOpen` IsNowOn)
      (goto _label_2))))

(event `self.ReceiveBeginPlay`
  (goto _label_3 :!via `SetNewTime`))

(fn `PositionOfHinge`
  (params (`Hinge Number` :type Integer))
  (returns (`Position of Hinge` :type "Vector Structure"))
  (locals (BufferCM :type "Float (double-precision)" :default 10.0))
  (bind _returnvalue (* (`self.Hinge Height`) 100.0))
  (bind (_relativescale3d_x _relativescale3d_y _relativescale3d_z) (`KismetMathLibrary.BreakVector` (`SceneComponent.RelativeScale3D` (`self.Mesh-Door`))))
  (return (`KismetMathLibrary.MakeVector` 0.0 0.0 (+ _returnvalue (* `Hinge Number` (/ (- (* _relativescale3d_z 100.0) (* _returnvalue 2.0)) (`KismetMathLibrary.Conv_IntToDouble` (- (`self.Number of Hinges`) 1))))))))

(fn `UserConstructionScript`
  (locals (DoorSize :type "Vector Structure" :default (0.0 0.0 0.0)))
  (bind _hinge_radius (`self.Hinge Radius`))
  (bind _thicc (`self.Thicc`))
  (bind _returnvalue (`KismetMathLibrary.MakeVector` (`self.Wide`) (`self.Thicc`) (`self.Tall`)))
  (bind _returnvalue_2 (* (`self.Thicc`) (`self.FrameThickMult`)))
  (bind _returnvalue_3 (* _thicc (`self.FrameThickMult`)))
  (bind _returnvalue_4 (* (`self.Tall`) (`self.FrameHeightMult`)))
  (bind _returnvalue_5 (`KismetMathLibrary.MakeTransform` (`KismetMathLibrary.MakeVector` (- (* _returnvalue_3 -50.0) (`self.FrameGap`)) (* _thicc 50.0) (* _returnvalue_4 50.0)) (struct) (`KismetMathLibrary.MakeVector` _returnvalue_3 _returnvalue_3 _returnvalue_4)))
  ;[1 1 1] Make Door
  (bind _output_get (set `local.DoorSize` _returnvalue))
  (`SceneComponent.K2_SetRelativeTransform` (`self.Mesh-Door`) (`KismetMathLibrary.MakeTransform` (* _output_get 50.0) (struct) _returnvalue) false true)
  (if (`self.Render door frame`)
    ;[1 1 1] Build door frame
    (`InstancedStaticMeshComponent.AddInstance` (`self.Mesh-Frame`) _returnvalue_5)
    (`InstancedStaticMeshComponent.AddInstance` (`self.Mesh-Frame`) (`KismetMathLibrary.MakeTransform` (`KismetMathLibrary.MakeVector` (+ (* (`self.Wide`) 100.0) (* (`self.Thicc`) (`self.FrameThickMult`) 50.0) (`self.FrameGap`)) (.y (.location _returnvalue_5)) (.z (.location _returnvalue_5))) (struct) (.scale _returnvalue_5)))
    (`InstancedStaticMeshComponent.AddInstance` (`self.Mesh-Frame`) (`KismetMathLibrary.MakeTransform` (`KismetMathLibrary.MakeVector` (* (`self.Wide`) 50.0) (* (`self.Thicc`) 50.0) (+ (* (`self.Tall`) 100.0) (* _returnvalue_2 50.0) (`self.FrameGap`))) (struct) (`KismetMathLibrary.MakeVector` (* (`self.Wide`) 1.5) _returnvalue_2 _returnvalue_2))))
  ;[1 1 1] Make Hinges
  (for _index (range (`self.Number of Hinges`))
    (bind _position_of_hinge (`self.PositionOfHinge` _index))
    (`InstancedStaticMeshComponent.AddInstance` (`self.Mesh-Hinge`) (`KismetMathLibrary.MakeTransform` _position_of_hinge (struct) (`KismetMathLibrary.MakeVector` _hinge_radius _hinge_radius (`self.Hinge Height`))))))