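; Tiki torch actor that lights or extinguishes by showing or hiding its point light and flame particle system together.
; A shared TurnLight function stores the on state and applies visibility, and the construction script runs it to preview the initial state.
; A Toggle event sets the state directly, while player interaction flips it only when CanPlayerChange allows.
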(event `/Game/Blueprints/Interface/ITriggerOrToggle.Toggle`
  (params (IsNowOn :type Boolean))
  (`self.Turn Light` IsNowOn))

(event `/Game/Blueprints/Interface/IPlayerCanLookAtAndInteractWith.PlayerWantsToInteract`
  (params (PlayerCharacter :type "/Game/Blueprints/PlayerAndGame/PlayerCharacter Object Reference"))
  (if (`self.Can Player Change`)
    (`self.Turn Light` (not (`self.IsOn`)))))

(fn `Turn Light`
  (params (`On?` :type Boolean))
  (bind _output_get (set `self.IsOn` `On?`))
  (`SceneComponent.SetVisibility` (`self.PointLight`) _output_get false)
  (`SceneComponent.SetVisibility` (`self.ParticleSystem`) _output_get false))

(fn `UserConstructionScript`
  (`self.Turn Light` (`self.IsOn`)))